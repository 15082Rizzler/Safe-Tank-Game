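; BP_Spawner_Enemy_Soldier is a spawner actor that keeps one BP_Enemy_Soldier in play, starting on BeginPlay.
; SpawnSoldier loops through delayed self-calls, rechecking periodically while its soldier is valid, otherwise spawning a replacement and waiting a random interval.
; Soldiers take the spawner's X, Y and rotation with a fixed Z height and undefined collision handling.
; An author note reports that spawning fails, though the same logic works for ammo and tank spawners.
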(event `self.ReceiveBeginPlay`
  ; To Vinh: If your reading this, I tried to set this up to spawn enemy soldiers, but for some reason it won't spawn them, despite this exact code working perfectly with ammo spawners and enemy tank spawners.
  (`self.Spawn Soldier`))

(event `Spawn Soldier`
  (bind (_returnvalue_x _returnvalue_y) (`KismetMathLibrary.BreakVector` (`self.K2_GetActorLocation`)))
  ; To Vinh: If your reading this, I tried to set this up to spawn enemy soldiers, but for some reason it won't spawn them, despite this exact code working perfectly with ammo spawners and enemy tank spawners.
  (`/Engine/EditorBlueprintResources/StandardMacros.IsValid` (`self.My Soldier`)
    (:`Is Valid`
      (`KismetSystemLibrary.Delay` 5.0)
      (`self.Spawn Soldier`))
    (:`Is Not Valid`
      (bind _returnvalue (`|SpawnActorFromClass` "/Game/Blueprints/BP_Enemy_Soldier.BP_Enemy_Soldier_C" (`KismetMathLibrary.MakeTransform` (`KismetMathLibrary.MakeVector` _returnvalue_x _returnvalue_y 21.0) (`self.K2_GetActorRotation`)) "Undefined" "MultiplyWithRoot" null null))
      (set `self.My Soldier` _returnvalue)
      (`KismetSystemLibrary.Delay` (`KismetMathLibrary.RandomFloatInRange` 10.0 20.0))
      (`self.Spawn Soldier`))))

(fn `UserConstructionScript`)