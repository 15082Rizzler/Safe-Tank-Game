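; AI controller for the enemy soldier that runs its behavior tree on possession and feeds it what perception detects.
; Sensing a Player-tagged actor sets the line-of-sight and Player blackboard keys and cancels the forget timer.
; Any other perception update starts that timer, which clears both keys when it expires.
; A Reload event re-enables the CanFire key after a short delay, and a helper function supplies blackboard access.
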(event `Reload`
  (bind (_blackboard _value_name) (`self.Func_BBData` "CanFire"))
  (`KismetSystemLibrary.Delay` 0.15)
  (`BlackboardComponent.SetValueAsBool` _blackboard _value_name true))

(event `self.ReceivePossess`
  (params (PossessedPawn :type "Pawn Object Reference"))
  (`self.RunBehaviorTree` "/Game/AI/BT_Enemy_Soldier.BT_Enemy_Soldier"))

(event `self.AIPerception.OnTargetPerceptionUpdated`
  (params (Actor :type "Actor Object Reference") (Stimulus :type "AIStimulus Structure"))
  (bind (_blackboard _value_name) (`self.Func_BBData` "Player"))
  (bind (_blackboard_2 _value_name_2) (`self.Func_BBData` "HasLineOfSight"))
  (if (and (`self.ActorHasTag` Actor "Player") (`.bSuccessfullySensed` (break `AIStimulus` Stimulus)))
    (`KismetSystemLibrary.K2_ClearAndInvalidateTimerHandle` (`self.Enemy Timer`))
    (`BlackboardComponent.SetValueAsBool` _blackboard_2 _value_name_2 true)
    (`BlackboardComponent.SetValueAsObject` _blackboard _value_name Actor)
    (else
      (bind _returnvalue (`KismetSystemLibrary.K2_SetTimerDelegate` (delegate `Start Enemy Timer`) (`self.LineOfSightTimer`)))
      (set `self.Enemy Timer` _returnvalue))))

(event `Start Enemy Timer`
  (bind (_blackboard _value_name) (`self.Func_BBData` "HasLineOfSight"))
  (bind (_blackboard_2 _value_name_2) (`self.Func_BBData` "Player"))
  (`BlackboardComponent.SetValueAsBool` _blackboard _value_name false)
  (`BlackboardComponent.SetValueAsObject` _blackboard_2 _value_name_2 null))

(fn `Func_BBData`
  (params (`BBValue Name` :type Name))
  (returns (Blackboard :type "BlackboardComponent Object Reference") (`Value Name` :type Name))
  (return (`AIBlueprintHelperLibrary.GetBlackboard` null) (`KismetSystemLibrary.MakeLiteralName` `BBValue Name`)))

(fn `UserConstructionScript`)