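; Spawner actor that keeps one enemy tank in play, creating a BP_Enemy_Tank on BeginPlay and replacing it once it is gone.
; SpawnTank re-calls itself after delays as a polling loop, waiting briefly while MyTank is valid and a random longer interval after each spawn.
; New tanks take the spawner's XY position and rotation at a fixed height.
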(event `self.ReceiveBeginPlay`
  (`self.Spawn Tank`))

(event `Spawn Tank`
  (bind (_returnvalue_x _returnvalue_y) (`KismetMathLibrary.BreakVector` (`self.K2_GetActorLocation`)))
  (`/Engine/EditorBlueprintResources/StandardMacros.IsValid` (`self.MyTank`)
    (:`Is Valid`
      (`KismetSystemLibrary.Delay` 5.0)
      (`self.Spawn Tank`))
    (:`Is Not Valid`
      (bind _returnvalue (`|SpawnActorFromClass` "/Game/Blueprints/BP_Enemy_Tank.BP_Enemy_Tank_C" (`KismetMathLibrary.MakeTransform` (`KismetMathLibrary.MakeVector` _returnvalue_x _returnvalue_y 21.0) (`self.K2_GetActorRotation`)) "Undefined" "MultiplyWithRoot" null null))
      (set `self.MyTank` _returnvalue)
      (`KismetSystemLibrary.Delay` (`KismetMathLibrary.RandomFloatInRange` 10.0 20.0))
      (`self.Spawn Tank`))))

(fn `UserConstructionScript`)