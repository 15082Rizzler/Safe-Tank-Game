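; Spawner actor that keeps one BP_Shell_Pickup available at its location, replacing it once it is gone.
; A self-calling SpawnTank event, which spawns shells despite its name, starts on BeginPlay and spawns at a fixed height with the spawner's rotation.
; After each spawn it waits a random few minutes, then polls every few seconds until the stored pickup is invalid before spawning again.
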(event `self.ReceiveBeginPlay`
  (`self.Spawn Tank`))

(event `Spawn Tank`
  (bind (_returnvalue_x _returnvalue_y) (`KismetMathLibrary.BreakVector` (`self.K2_GetActorLocation`)))
  (`/Engine/EditorBlueprintResources/StandardMacros.IsValid` (`self.My Shell`)
    (:`Is Valid`
      (`KismetSystemLibrary.Delay` 5.0)
      (`self.Spawn Tank`))
    (:`Is Not Valid`
      (bind _returnvalue (`|SpawnActorFromClass` "/Game/Blueprints/BP_Shell_Pickup.BP_Shell_Pickup_C" (`KismetMathLibrary.MakeTransform` (`KismetMathLibrary.MakeVector` _returnvalue_x _returnvalue_y 21.0) (`self.K2_GetActorRotation`)) "Undefined" "MultiplyWithRoot" null null))
      (set `self.My Shell` _returnvalue)
      (`KismetSystemLibrary.Delay` (`KismetMathLibrary.RandomFloatInRange` 120.0 180.0))
      (`self.Spawn Tank`))))

(fn `UserConstructionScript`)