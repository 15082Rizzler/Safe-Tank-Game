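; Enemy soldier, driven by an AI controller, that the player tank can kill for score.
; On BeginPlay it finds the player tank and writes it to its Blackboard's "Player" key.
; Box overlaps with tagged player shells or bullets spawn an explosion, destroy the projectile and call Perish.
; Perish destroys the AI controller, swaps the Sphere material and updates score, leaving the body; its controller check prevents repeat scoring.
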(event `self.ReceiveTick`
  (params (DeltaSeconds :type "Float (single-precision)")))

(event `self.ReceiveBeginPlay`
  (bind (_returnvalue _returnvalue2) (`self.Func_BBData` "Player"))
  (bind _returnvalue_2 (`GameplayStatics.GetActorOfClass` "/Game/Blueprints/BP_PlayerTank.BP_PlayerTank_C"))
  (bind _output_get (set `self.Player Ref` _returnvalue_2))
  (`BlackboardComponent.SetValueAsObject` _returnvalue _returnvalue2 _output_get))

(event `self.Box.OnComponentBeginOverlap`
  (params (OverlappedComponent :type "PrimitiveComponent Object Reference") (OtherActor :type "Actor Object Reference") (OtherComp :type "PrimitiveComponent Object Reference") (OtherBodyIndex :type Integer) (bFromSweep :type Boolean) (SweepResult :type "HitResult Structure (by ref)"))
  (if (> (`KismetArrayLibrary.Array_Find` (`Actor.Tags` OtherActor) "PlayerShell") -1)
    (`NiagaraFunctionLibrary.SpawnSystemAtLocation` "/Game/VFX/NS_SmallExplosion.NS_SmallExplosion" :!label _label)
    (`GameplayStatics.PlaySoundAtLocation` "/Game/Sounds/SW_Explosion.SW_Explosion" (`self.K2_GetActorLocation` OtherActor) (struct) 1.0 1.0 0.0 null null null null)
    (`self.K2_DestroyActor` OtherActor)
    (`self.Perish`)
    (elif (> (`KismetArrayLibrary.Array_Find` (`Actor.Tags` OtherActor) "PlayerBullet") -1)
      (goto _label))))

(event `Perish`
  (bind _returnvalue (`AIBlueprintHelperLibrary.GetAIController` self))
  (`/Engine/EditorBlueprintResources/StandardMacros.IsValid` _returnvalue
    (:`Is Valid`
      (bind _output_get (set `self.Delete This AIController` _returnvalue))
      (`Controller.UnPossess` _output_get)
      (`self.K2_DestroyActor` _output_get)
      (`PrimitiveComponent.SetMaterial` (`self.Sphere`) 0 "/Game/Materials/MAT_BaseNonMetalic.MAT_BaseNonMetalic")
      (bind _returnvalue_2 (`GameplayStatics.GetActorOfClass` "/Game/Blueprints/BP_PlayerTank.BP_PlayerTank_C"))
      (`/Game/Blueprints/BP_PlayerTank.Update Score` _returnvalue_2))))

(fn `Func_BBData`
  (params (KeyName :type Name))
  (returns (ReturnValue :type "BlackboardComponent Object Reference") (ReturnValue2 :type Name))
  (return (`AIBlueprintHelperLibrary.GetBlackboard` (`AIBlueprintHelperLibrary.GetAIController` self)) (`KismetSystemLibrary.MakeLiteralName` KeyName)))

(fn `UserConstructionScript`)