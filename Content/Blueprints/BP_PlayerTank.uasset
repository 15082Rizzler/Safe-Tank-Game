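; Player tank pawn with Enhanced Input driving, five gears, engine toggle, score, and shell-hit damage leading to a death screen.
; Driving and turning are mutually exclusive and require a running engine.
; A timeline-animated toggle switches between the manually reloaded main gun and a rate-limited machine gun turret.
; Engine, gear and firing noise set every BP_Enemy_Tank's hearing radius, while state changes are pushed to BP_MainHUD.
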(event `self.Box collider.OnComponentBeginOverlap`
  (params (OverlappedComponent :type "PrimitiveComponent Object Reference") (OtherActor :type "Actor Object Reference") (OtherComp :type "PrimitiveComponent Object Reference") (OtherBodyIndex :type Integer) (bFromSweep :type Boolean) (SweepResult :type "HitResult Structure (by ref)"))
  ;[0.07292 0 0.00694 0.5] Get hurt by enemy shells and Die if integrity is depleated
  (if (> (`KismetArrayLibrary.Array_Find` (`Actor.Tags` OtherActor) "EnemyShell") -1)
    (`NiagaraFunctionLibrary.SpawnSystemAtLocation` "/Game/VFX/NS_SmallExplosion.NS_SmallExplosion" (`self.K2_GetActorLocation` OtherActor))
    (`GameplayStatics.PlaySoundAtLocation` "/Game/Sounds/SW_Explosion.SW_Explosion" (`self.K2_GetActorLocation` OtherActor) (struct) 1.0 1.0 0.0 null null null null)
    (`self.K2_DestroyActor` OtherActor)
    (bind _output_get (set `self.Tank Integrity` (- (`self.Tank Integrity`) 1)))
    (bind _asbp_main_hud (cast `/Game/UI/BP_MainHUD` (`PlayerController.GetHUD` (`GameplayStatics.GetPlayerController` 0))))
    (`/Game/UI/BP_MainHUD.HUD_Update Integrity Meter` _asbp_main_hud _output_get)
    (if (== (`self.Tank Integrity`) 0)
      (`EnhancedInputSubsystemInterface.RemoveMappingContext` (pcsubsystem `EnhancedInputLocalPlayerSubsystem` (`GameplayStatics.GetPlayerController` 0)) "/Game/Input/IMC_Tank.IMC_Tank" (struct))
      (`PrimitiveComponent.SetMaterial` (`self.Gun`) 0 "/Game/Materials/MAT_BaseNonMetalic.MAT_BaseNonMetalic")
      (`PrimitiveComponent.SetMaterial` (`self.Gun nozzle`) 0 "/Game/Materials/MAT_BaseNonMetalic.MAT_BaseNonMetalic")
      (bind _returnvalue (`AddComponent|NODE_AddNiagaraComponent-0`))
      (`NiagaraComponent.SetAsset` _returnvalue "/Game/VFX/NS_Explosion.NS_Explosion" true)
      (set `PlayerController.bShowMouseCursor` true (`GameplayStatics.GetPlayerController` 0))
      (`/Game/UI/BP_MainHUD.HUD_Death Screen` _asbp_main_hud))))

(event `Update Score`
  ;[0 0.15 0.01016 0.999] Change the score. Usually called by enemies upon their death.
  (bind _output_get (set `self.Score` (+ (`self.Score`) 1)))
  (bind _asbp_main_hud (cast `/Game/UI/BP_MainHUD` (`PlayerController.GetHUD` (`GameplayStatics.GetPlayerController` 0))))
  (`/Game/UI/BP_MainHUD.HUD_Set Score` _asbp_main_hud _output_get))

(event `EnhancedInput|/Game/Input/IA_MuteEnemyMovement`
  (params (ActionValue :type Boolean) (ElapsedSeconds :type "Float (double-precision)") (TriggeredSeconds :type "Float (double-precision)") (InputAction :type "InputAction Object Reference" :default "/Game/Input/IA_MuteEnemyMovement.IA_MuteEnemyMovement"))
  ; Mute Enemy Movement
  (:`Started`
    (`/Engine/EditorBlueprintResources/StandardMacros.FlipFlop`
      (:`A`
        (set `self.Mute Enemy Movement` true))
      (:`B`
        (set `self.Mute Enemy Movement` false)))))

(event `EnhancedInput|/Game/Input/IA_1stGear`
  (params (ActionValue :type Boolean) (ElapsedSeconds :type "Float (double-precision)") (TriggeredSeconds :type "Float (double-precision)") (InputAction :type "InputAction Object Reference" :default "/Game/Input/IA_1stGear.IA_1stGear"))
  ;[0 0.3218 1] Change gears
  (:`Started`
    (set `self.Gear` 1)
    (set `self.Gear multiplier` (0.4 0.4 0.0))
    (set `self.Gear Noise Modifier` 150.0)
    (bind _asbp_main_hud (cast `/Game/UI/BP_MainHUD` (`PlayerController.GetHUD` (`GameplayStatics.GetPlayerController` 0))))
    (`/Game/UI/BP_MainHUD.HUD_Update Gears` _asbp_main_hud (`self.Gear`))
    (`self.Func_UpdateDisplay` 5 1)))

(event `NT4`
  (bind _turret (`self.Turret`))
  (bind (_relativelocation_x _relativelocation_y) (`KismetMathLibrary.BreakVector` (`SceneComponent.RelativeLocation` _turret)))
  ;[1 0.2977 0.9734 0.5] Switching to the Machine gun turret + Turret activation animation
  (bind (_direction _upward_movement _change_turret_scale) (`Timeline|Inverse TurretAnimation` :!via `SetNewTime` :!label _label)
    (:`Update`
      (`SceneComponent.K2_SetRelativeLocation` _turret (`KismetMathLibrary.MakeVector` _relativelocation_x _relativelocation_y (.z _upward_movement)) false false))
    (:`Finished`
      (set `self.Using Turret` false)
      (set `self.Turret Anim In progress` false)
      (`KismetSystemLibrary.PrintString` "Done again"))))

(event `NT3`
  (bind _turretnozzle (`self.TurretNozzle`))
  (bind (_relativescale3d_x _relativescale3d_y _relativescale3d_z) (`KismetMathLibrary.BreakVector` (`SceneComponent.RelativeScale3D` _turretnozzle)))
  ;[1 0.2977 0.9734 0.5] Switching to the Machine gun turret + Turret activation animation
  (bind (_direction _scaleturretnozzle) (`Timeline|Inverse ExtendTurretGun` :!via `SetNewTime` :!label _label_2)
    (:`Update`
      (`SceneComponent.SetRelativeScale3D` _turretnozzle (`KismetMathLibrary.MakeVector` (.x _scaleturretnozzle) _relativescale3d_y _relativescale3d_z)))
    (:`Finished`
      (goto _label :!via `PlayFromStart`))))

(event `EnhancedInput|/Game/Input/IA_2ndGear`
  (params (ActionValue :type Boolean) (ElapsedSeconds :type "Float (double-precision)") (TriggeredSeconds :type "Float (double-precision)") (InputAction :type "InputAction Object Reference" :default "/Game/Input/IA_2ndGear.IA_2ndGear"))
  ;[0 0.3218 1] Change gears
  (:`Started`
    (set `self.Gear` 2)
    (set `self.Gear multiplier` (0.7 0.7 0.0))
    (set `self.Gear Noise Modifier` 250.0)
    (bind _asbp_main_hud (cast `/Game/UI/BP_MainHUD` (`PlayerController.GetHUD` (`GameplayStatics.GetPlayerController` 0))))
    (`/Game/UI/BP_MainHUD.HUD_Update Gears` _asbp_main_hud (`self.Gear`))
    (`self.Func_UpdateDisplay` 6 1)))

(event `self.ReceiveBeginPlay`
  ;[1 1 1] BeginPlay
  (`EnhancedInputSubsystemInterface.AddMappingContext` (pcsubsystem `EnhancedInputLocalPlayerSubsystem` (`GameplayStatics.GetPlayerController` 0)) "/Game/Input/IMC_Tank.IMC_Tank" 0 (struct))
  (`self.Func_CreateSounds`)
  (bind _asbp_main_hud (cast `/Game/UI/BP_MainHUD` (`PlayerController.GetHUD` (`GameplayStatics.GetPlayerController` 0))))
  (`/Game/UI/BP_MainHUD.HUD_Engine check` _asbp_main_hud (`self.Is engine on?`))
  (`/Game/UI/BP_MainHUD.HUD_Shells left` _asbp_main_hud (`self.Shells left`))
  (`/Game/UI/BP_MainHUD.HUD_Reload` _asbp_main_hud (`self.Is turret loaded?`))
  (`/Game/UI/BP_MainHUD.HUD_Update Gears` _asbp_main_hud (`self.Gear`))
  (`/Game/UI/BP_MainHUD.HUD_Update Integrity Meter` _asbp_main_hud (`self.Tank Integrity`))
  (`/Game/UI/BP_MainHUD.HUD_Set Score` _asbp_main_hud (`self.Score`))
  (`/Game/UI/BP_MainHUD.HUD_Check Bullet Count` _asbp_main_hud (`self.Turret Ammo`))
  (bind _returnvalue (`GameplayStatics.GetActorOfClass` "/Game/Blueprints/BP_PlayerRefBroadcaster.BP_PlayerRefBroadcaster_C"))
  (`/Game/Blueprints/BP_PlayerRefBroadcaster.SetupRefBroadcast` _returnvalue self))

(event `EnhancedInput|/Game/Input/IA_ToggleTurret`
  (params (ActionValue :type Boolean) (ElapsedSeconds :type "Float (double-precision)") (TriggeredSeconds :type "Float (double-precision)") (InputAction :type "InputAction Object Reference" :default "/Game/Input/IA_ToggleTurret.IA_ToggleTurret"))
  (bind _turretnozzle (`self.TurretNozzle`))
  (bind _turret (`self.Turret`))
  (bind (_relativescale3d_x _relativescale3d_y _relativescale3d_z) (`KismetMathLibrary.BreakVector` (`SceneComponent.RelativeScale3D` _turretnozzle)))
  (bind (_relativelocation_x _relativelocation_y) (`KismetMathLibrary.BreakVector` (`SceneComponent.RelativeLocation` _turret)))
  ;[1 0.2977 0.9734 0.5] Switching to the Machine gun turret + Turret activation animation
  (:`Started`
    (if (not (`self.Turret Anim In progress`))
      (set `self.Turret Anim In progress` true)
      (if (`self.Is Turret On?`)
        (set `self.Is Turret On?` false)
        (goto _label_2)
        (else
          (set `self.Using Turret` true)
          (bind (_direction _upward_movement) (`Timeline|TurretAnimation` :!via `PlayFromStart` :!label _label_3)
            (:`Update`
              (`SceneComponent.K2_SetRelativeLocation` _turret (`KismetMathLibrary.MakeVector` _relativelocation_x _relativelocation_y (.z _upward_movement)) false false))
            (:`Finished`
              (bind (_direction_2 _scaleturretnozzle) (`Timeline|ExtendTurretGun` :!via `PlayFromStart` :!label _label_4)
                (:`Update`
                  (`SceneComponent.SetRelativeScale3D` _turretnozzle (`KismetMathLibrary.MakeVector` (.x _scaleturretnozzle) _relativescale3d_y _relativescale3d_z)))
                (:`Finished`
                  (set `self.Is Turret On?` true)
                  (set `self.Turret Anim In progress` false)
                  (`KismetSystemLibrary.PrintString` "Done"))))))))))

(event `EnhancedInput|/Game/Input/IA_3rdGear`
  (params (ActionValue :type Boolean) (ElapsedSeconds :type "Float (double-precision)") (TriggeredSeconds :type "Float (double-precision)") (InputAction :type "InputAction Object Reference" :default "/Game/Input/IA_3rdGear.IA_3rdGear"))
  ;[0 0.3218 1] Change gears
  (:`Started`
    (set `self.Gear` 3)
    (set `self.Gear multiplier` (1.0 1.0 0.0))
    (set `self.Gear Noise Modifier` 350.0)
    (bind _asbp_main_hud (cast `/Game/UI/BP_MainHUD` (`PlayerController.GetHUD` (`GameplayStatics.GetPlayerController` 0))))
    (`/Game/UI/BP_MainHUD.HUD_Update Gears` _asbp_main_hud (`self.Gear`))
    (`self.Func_UpdateDisplay` 7 1)))

(event `EnhancedInput|/Game/Input/IA_MoveUpDown`
  (params (ActionValue :type "Float (double-precision)") (ElapsedSeconds :type "Float (double-precision)") (TriggeredSeconds :type "Float (double-precision)") (InputAction :type "InputAction Object Reference" :default "/Game/Input/IA_MoveUpDown.IA_MoveUpDown"))
  (bind _sound_tanktreadsmoving (`self.SOUND_TankTreadsMoving`))
  ;[1 0.756 0.1085] Moving
  (:`Triggered`
    (if (`self.Is engine on?`)
      (if (not (`self.Turning`))
        (set `self.Driving` true)
        (if (> ActionValue 0.0)
          (`PawnMovementComponent.AddInputVector` (`self.FloatingPawnMovement`) (* (`SceneComponent.GetForwardVector` (`self.Arrow`)) (* (0.5 0.5 0.0) (`self.Gear multiplier`))) false)
          (`ActorComponent.SetActive` _sound_tanktreadsmoving true false)
          (`self.Func_UpdateDisplay` 1)
          (else
            (`PawnMovementComponent.AddInputVector` (`self.FloatingPawnMovement`) (* (`KismetMathLibrary.GreaterGreater_VectorRotator` (`SceneComponent.GetForwardVector` (`self.Arrow`)) (struct :`Yaw` 180.0)) (* (0.5 0.5 0.0) (`self.Gear multiplier`))) false)
            (`ActorComponent.SetActive` _sound_tanktreadsmoving true false)
            (`self.Func_UpdateDisplay` 2))))))
  (:`Started`
    (`self.Func_MoveNoise` ActionValue))
  (:`Completed`
    (`ActorComponent.SetActive` (`self.SOUND_TankTreadsMoving`) false false)
    (if (`self.Is engine on?`)
      (set `self.Driving` false)
      (bind _output_get (set `self.Noise Level` (`self.Engine Passive Noise`)))
      (`self.Func_UpdateNoise` _output_get)
      (`self.Func_UpdateDisplay` 0))))

(event `NT1`
  ;[1 0.2977 0.9734 0.5] Switching to the Machine gun turret + Turret activation animation
  (goto _label_3 :!via `SetNewTime`))

(event `EnhancedInput|/Game/Input/IA_4thGear`
  (params (ActionValue :type Boolean) (ElapsedSeconds :type "Float (double-precision)") (TriggeredSeconds :type "Float (double-precision)") (InputAction :type "InputAction Object Reference" :default "/Game/Input/IA_4thGear.IA_4thGear"))
  ;[0 0.3218 1] Change gears
  (:`Started`
    (set `self.Gear` 4)
    (set `self.Gear multiplier` (1.3 1.3 0.0))
    (set `self.Gear Noise Modifier` 450.0)
    (bind _asbp_main_hud (cast `/Game/UI/BP_MainHUD` (`PlayerController.GetHUD` (`GameplayStatics.GetPlayerController` 0))))
    (`/Game/UI/BP_MainHUD.HUD_Update Gears` _asbp_main_hud (`self.Gear`))
    (`self.Func_UpdateDisplay` 8 1)))

(event `NT2`
  ;[1 0.2977 0.9734 0.5] Switching to the Machine gun turret + Turret activation animation
  (goto _label_4 :!via `SetNewTime`))

(event `EnhancedInput|/Game/Input/IA_5thGear`
  (params (ActionValue :type Boolean) (ElapsedSeconds :type "Float (double-precision)") (TriggeredSeconds :type "Float (double-precision)") (InputAction :type "InputAction Object Reference" :default "/Game/Input/IA_5thGear.IA_5thGear"))
  ;[0 0.3218 1] Change gears
  (:`Started`
    (set `self.Gear` 5)
    (set `self.Gear multiplier` (1.6 1.6 0.0))
    (set `self.Gear Noise Modifier` 550.0)
    (bind _asbp_main_hud (cast `/Game/UI/BP_MainHUD` (`PlayerController.GetHUD` (`GameplayStatics.GetPlayerController` 0))))
    (`/Game/UI/BP_MainHUD.HUD_Update Gears` _asbp_main_hud (`self.Gear`))
    (`self.Func_UpdateDisplay` 9 1)))

(event `EnhancedInput|/Game/Input/IA_ToggleEngine`
  (params (ActionValue :type Boolean) (ElapsedSeconds :type "Float (double-precision)") (TriggeredSeconds :type "Float (double-precision)") (InputAction :type "InputAction Object Reference" :default "/Game/Input/IA_ToggleEngine.IA_ToggleEngine"))
  ;[0.5604 1 0.7338] Turn engine on/off
  (:`Started`
    (if (`self.Toggle engine mode`)
      (if (`self.Toggle engine mode 2`)
        (set `self.Toggle engine mode 2` false)
        (`KismetSystemLibrary.Delay` 1.4)
        (set `self.Is engine on?` true)
        (bind _asbp_main_hud (cast `/Game/UI/BP_MainHUD` (`PlayerController.GetHUD` (`GameplayStatics.GetPlayerController` 0))))
        (`/Game/UI/BP_MainHUD.HUD_Engine check` _asbp_main_hud (`self.Is engine on?`))
        (bind _output_get (set `self.Noise Level` (`self.Engine Passive Noise`)))
        (`self.Func_UpdateNoise` _output_get)
        (set `self.Toggle engine mode` false))
      (elif (not (`self.Toggle engine mode 2`))
        (set `self.Toggle engine mode 2` true)
        (set `self.Is engine on?` false)
        (set `self.Driving` false)
        (set `self.Turning` false)
        (bind _asbp_main_hud_2 (cast `/Game/UI/BP_MainHUD` (`PlayerController.GetHUD` (`GameplayStatics.GetPlayerController` 0))))
        (`/Game/UI/BP_MainHUD.HUD_Engine check` _asbp_main_hud_2 (`self.Is engine on?`))
        (bind _output_get_2 (set `self.Noise Level` 0.1))
        (`self.Func_UpdateNoise` _output_get_2)
        (set `self.Toggle engine mode` true)))))

(event `EnhancedInput|/Game/Input/IA_MoveLeftRight`
  (params (ActionValue :type "Float (double-precision)") (ElapsedSeconds :type "Float (double-precision)") (TriggeredSeconds :type "Float (double-precision)") (InputAction :type "InputAction Object Reference" :default "/Game/Input/IA_MoveLeftRight.IA_MoveLeftRight"))
  (bind _sound_tanktreadsrotating (`self.SOUND_TankTreadsRotating`))
  (bind _arrow (`self.Arrow`))
  (bind _tank (`self.Tank`))
  ;[0.4982 0.2768 1] Turning
  (:`Triggered`
    (if (`self.Is engine on?`)
      (if (not (`self.Driving`))
        (set `self.Turning` true)
        (if (> ActionValue 0.0)
          (`SceneComponent.K2_AddLocalRotation` _arrow (struct :`Yaw` 1.0) false false)
          (`SceneComponent.K2_AddLocalRotation` _tank (struct :`Yaw` 1.0) false false)
          (`ActorComponent.SetActive` _sound_tanktreadsrotating true false)
          (`self.Func_UpdateDisplay` 4)
          (else
            (`SceneComponent.K2_AddLocalRotation` _arrow (struct :`Yaw` -1.0) false false)
            (`SceneComponent.K2_AddLocalRotation` _tank (struct :`Yaw` -1.0) false false)
            (`ActorComponent.SetActive` _sound_tanktreadsrotating true false)
            (`self.Func_UpdateDisplay` 3))))))
  (:`Completed`
    (`ActorComponent.SetActive` (`self.SOUND_TankTreadsRotating`) false false)
    (if (`self.Is engine on?`)
      (set `self.Turning` false)
      (`self.Func_UpdateDisplay` 0))))

(event `EnhancedInput|/Game/Input/IA_Reload`
  (params (ActionValue :type Boolean) (ElapsedSeconds :type "Float (double-precision)") (TriggeredSeconds :type "Float (double-precision)") (InputAction :type "InputAction Object Reference" :default "/Game/Input/IA_Reload.IA_Reload"))
  ;[1 0.3651 0] Reload turret
  (:`Started`
    (if (not (`self.Is turret loaded?`))
      (bind _asbp_main_hud (cast `/Game/UI/BP_MainHUD` (`PlayerController.GetHUD` (`GameplayStatics.GetPlayerController` 0))))
      (`/Game/UI/BP_MainHUD.HUD_Reload` _asbp_main_hud (`self.Is turret loaded?`))
      (`KismetSystemLibrary.Delay` (`KismetMathLibrary.RandomFloatInRange` 3.2 6.8))
      (bind _output_get (set `self.Is turret loaded?` true))
      (`/Game/UI/BP_MainHUD.HUD_Reload` _asbp_main_hud _output_get))))

(event `EnhancedInput|/Game/Input/IA_RotateGun`
  (params (ActionValue :type "Float (double-precision)") (ElapsedSeconds :type "Float (double-precision)") (TriggeredSeconds :type "Float (double-precision)") (InputAction :type "InputAction Object Reference" :default "/Game/Input/IA_RotateGun.IA_RotateGun"))
  (bind _sound_turretrotation (`self.SOUND_TurretRotation`))
  (bind _sound_turretrotation_2 (`self.SOUND_TurretRotation`))
  ;[1 0.3604 0.6837] Rotate Gun
  (:`Triggered`
    (if (`self.Is engine on?`)
      (if (`self.Using Turret`)
        (if (`self.Is Turret On?`)
          (if (> ActionValue 0.0)
            (`SceneComponent.K2_AddLocalRotation` (`self.Turret`) (struct :`Yaw` 1.0) false false)
            (`ActorComponent.SetActive` _sound_turretrotation true false)
            (else
              (`SceneComponent.K2_AddLocalRotation` (`self.Turret`) (struct :`Yaw` -1.0) false false)
              (`ActorComponent.SetActive` _sound_turretrotation true false))))
        (elif (> ActionValue 0.0)
          (`SceneComponent.K2_AddLocalRotation` (`self.Gun`) (struct :`Yaw` 1.0) false false)
          (`ActorComponent.SetActive` _sound_turretrotation_2 true false)
          (else
            (`SceneComponent.K2_AddLocalRotation` (`self.Gun`) (struct :`Yaw` -1.0) false false)
            (`ActorComponent.SetActive` _sound_turretrotation_2 true false))))))
  (:`Completed`
    (`ActorComponent.SetActive` (`self.SOUND_TurretRotation`) false false)))

(event `Turret Fire Rate Timer`
  ;[1 0.125 0.125] Shooting
  ;;[0.724 0 0 0.5] Turret fire rate determiner
  (`KismetSystemLibrary.Delay` (`self.Turret Fire Rate`))
  (set `self.Turret Can Shoot` true))

(event `EnhancedInput|/Game/Input/IA_ShootTank`
  (params (ActionValue :type Boolean) (ElapsedSeconds :type "Float (double-precision)") (TriggeredSeconds :type "Float (double-precision)") (InputAction :type "InputAction Object Reference" :default "/Game/Input/IA_ShootTank.IA_ShootTank"))
  ;[1 0.125 0.125] Shooting
  (:`Triggered`
    (if (`self.Is Turret On?`)
      (`|ExecutionSequence`
        (:`then_0`
          (set `self.Don't emit sound driving` true)
          (`KismetSystemLibrary.Delay` 0.2)
          (set `self.Don't emit sound driving` false))
        (:`then_1`
          (if (`self.Is engine on?`)
            (if (> (`self.Turret Ammo`) 0)
              (if (`self.Turret Can Shoot`)
                (`|SpawnActorFromClass` "/Game/Blueprints/BP_Shell.BP_Shell_C" (`KismetMathLibrary.MakeTransform` (`SceneComponent.K2_GetComponentLocation` (`self.ShootPointTurret`)) (`SceneComponent.K2_GetComponentRotation` (`self.Turret`))) "Undefined" "MultiplyWithRoot" null null)
                (set `self.Turret Can Shoot` false)
                (bind _output_get (set `self.Turret Ammo` (- (`self.Turret Ammo`) 1)))
                (`self.Turret Fire Rate Timer`)
                (bind _asbp_main_hud (cast `/Game/UI/BP_MainHUD` (`PlayerController.GetHUD` (`GameplayStatics.GetPlayerController` 0))))
                (`/Game/UI/BP_MainHUD.HUD_Check Bullet Count` _asbp_main_hud _output_get)
                (set `self.Just Fired` true)
                (bind _output_get_2 (set `self.Noise Level` 1050.0))
                (`GameplayStatics.PlaySoundAtLocation` "/Game/Sounds/SW_Tank_Shot.SW_Tank_Shot" (`self.K2_GetActorLocation`) (struct) 1.0 1.0 0.0 null null null null)
                (`self.Func_UpdateNoise` _output_get_2)
                (if (`self.Driving`)
                  (`KismetSystemLibrary.Delay` 0.2)
                  (set `self.Noise Level` (`self.Gear Noise Modifier`))
                  (`self.Func_UpdateNoise` 0.0)
                  (set `self.Just Fired` false)
                  (else
                    (`KismetSystemLibrary.Delay` 0.2)
                    (set `self.Noise Level` (`self.Engine Passive Noise`))
                    (`self.Func_UpdateNoise` 0.0)
                    (set `self.Just Fired` false))))))))))
  (:`Started`
    (if (not (`self.Is Turret On?`))
      (`|ExecutionSequence`
        (:`then_0`
          (set `self.Don't emit sound driving` true)
          (`KismetSystemLibrary.Delay` 0.2)
          (set `self.Don't emit sound driving` false))
        (:`then_1`
          (if (`self.Is engine on?`)
            (if (`self.Is turret loaded?`)
              (if (> (`self.Shells left`) 0)
                (`|SpawnActorFromClass` "/Game/Blueprints/BP_Shell.BP_Shell_C" (`KismetMathLibrary.MakeTransform` (`SceneComponent.K2_GetComponentLocation` (`self.ShootPoint`)) (`SceneComponent.K2_GetComponentRotation` (`self.Gun`))) "Undefined" "MultiplyWithRoot" null null)
                (set `self.Is turret loaded?` false)
                (bind _output_get_3 (set `self.Shells left` (- (`self.Shells left`) 1)))
                (bind _asbp_main_hud_2 (cast `/Game/UI/BP_MainHUD` (`PlayerController.GetHUD` (`GameplayStatics.GetPlayerController` 0))))
                (`/Game/UI/BP_MainHUD.HUD_Shells left` _asbp_main_hud_2 _output_get_3)
                (set `self.Just Fired` true)
                (bind _output_get_4 (set `self.Noise Level` 1050.0))
                (`GameplayStatics.PlaySoundAtLocation` "/Game/Sounds/SW_Tank_Shot.SW_Tank_Shot" (`self.K2_GetActorLocation`) (struct) 1.0 1.0 0.0 null null null null)
                (`self.Func_UpdateNoise` _output_get_4)
                (if (`self.Driving`)
                  (`KismetSystemLibrary.Delay` 0.2)
                  (set `self.Noise Level` (`self.Gear Noise Modifier`))
                  (`self.Func_UpdateNoise` 0.0)
                  (set `self.Just Fired` false)
                  (else
                    (`KismetSystemLibrary.Delay` 0.2)
                    (set `self.Noise Level` (`self.Engine Passive Noise`))
                    (`self.Func_UpdateNoise` 0.0)
                    (set `self.Just Fired` false)))))))))))

(fn `Func_CreateSounds`
  (bind _returnvalue (`GameplayStatics.SpawnSound2D` "/Game/Sounds/SW_Tank_Turret_Rotating.SW_Tank_Turret_Rotating" 1.0 1.0 0.0 null false false))
  (bind _output_get (set `self.SOUND_TurretRotation` _returnvalue))
  (`ActorComponent.SetActive` _output_get false false)
  (bind _returnvalue_2 (`GameplayStatics.SpawnSound2D` "/Game/Sounds/SW_Tank_Treads_Rotating.SW_Tank_Treads_Rotating" 1.0 1.0 0.0 null false false))
  (bind _output_get_2 (set `self.SOUND_TankTreadsRotating` _returnvalue_2))
  (`ActorComponent.SetActive` _output_get_2 false false)
  (bind _returnvalue_3 (`GameplayStatics.SpawnSound2D` "/Game/Sounds/SW_Tank_Treads_Moving.SW_Tank_Treads_Moving" 1.0 1.0 0.0 null false false))
  (bind _output_get_3 (set `self.SOUND_TankTreadsMoving` _returnvalue_3))
  (`ActorComponent.SetActive` _output_get_3 false false))

(fn `Func_MoveNoise`
  (params (`Action Value` :type "Float (double-precision)"))
  (if (> `Action Value` 0.0)
    (if (`self.Don't emit sound driving`)
      _
      (elif (not (`self.Just Fired`))
        (bind _output_get (set `self.Noise Level` (`self.Gear Noise Modifier`)))
        (`self.Func_UpdateNoise` _output_get)))
    (elif (`self.Don't emit sound driving`)
      _
      (elif (not (`self.Just Fired`))
        (bind _output_get_2 (set `self.Noise Level` (`self.Gear Noise Modifier`)))
        (`self.Func_UpdateNoise` _output_get_2)))))

(fn `Func_UpdateDisplay`
  (params (`Display ID` :type Integer) (`Display Mode` :type Integer))
  (bind _asbp_main_hud (cast `/Game/UI/BP_MainHUD` (`PlayerController.GetHUD` (`GameplayStatics.GetPlayerController` 0))))
  (if (== `Display Mode` 0)
    (`/Game/UI/BP_MainHUD.HUD_Change Display` _asbp_main_hud `Display ID`)
    (elif (== `Display Mode` 1)
      (`/Game/UI/BP_MainHUD.HUD_ChangeGearControls` _asbp_main_hud `Display ID`)
      (elif (== `Display Mode` 2)
        _))))

(fn `Func_UpdateNoise`
  (params (`Noise Input` :type "Float (double-precision)"))
  (bind _outactors (`GameplayStatics.GetAllActorsOfClass` "/Game/Blueprints/BP_Enemy_Tank.BP_Enemy_Tank_C"))
  (for _array_element _outactors
    (`/Game/Blueprints/BP_Enemy_Tank.Change Hearing Radius` _array_element `Noise Input`)))

(fn `UserConstructionScript`)