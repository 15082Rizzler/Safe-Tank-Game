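; Shell pickup actor that refills the player tank's ammunition when driven over.
; On overlap with BP_PlayerTank it adds a fixed number of shells to ShellsLeft and pushes the new count to BP_MainHUD through the local viewing player controller.
; It then plays a shotgun rack sound at its location and destroys itself, but only if the HUD cast succeeds.
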(event `self.ReceiveActorBeginOverlap`
  (params (OtherActor :type "Actor Object Reference"))
  (bind _asbp_player_tank (cast `/Game/Blueprints/BP_PlayerTank` OtherActor))
  (bind _output_get (set `/Game/Blueprints/BP_PlayerTank.Shells left` (+ (`/Game/Blueprints/BP_PlayerTank.Shells left` _asbp_player_tank) 3) _asbp_player_tank))
  (bind _asbp_main_hud (cast `/Game/UI/BP_MainHUD` (`PlayerController.GetHUD` (`Pawn.GetLocalViewingPlayerController` _asbp_player_tank))))
  (`/Game/UI/BP_MainHUD.HUD_Shells left` _asbp_main_hud _output_get)
  (`GameplayStatics.PlaySoundAtLocation` "/Game/Sounds/SW_Shotgun_Rack.SW_Shotgun_Rack" (`self.K2_GetActorLocation`) (struct) 1.0 1.0 0.0 null null null null)
  (`self.K2_DestroyActor`))

(fn `UserConstructionScript`)